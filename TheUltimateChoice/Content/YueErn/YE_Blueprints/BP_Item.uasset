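; BP_Item is an item actor that shows proximity-based interaction icons to the player.
; Two sphere collisions react only to player character 0: entering the outer sphere shows the outer icon, and entering the inner sphere swaps it for the inner icon.
; Leaving each sphere reverses that change.
; The construction script sets both sphere radii from variables; the graphs contain only icon visibility logic, with no interaction action.
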(event `self.innerSphereCollision.OnComponentBeginOverlap`
  (params (OverlappedComponent :type "PrimitiveComponent Object Reference") (OtherActor :type "Actor Object Reference") (OtherComp :type "PrimitiveComponent Object Reference") (OtherBodyIndex :type Integer) (bFromSweep :type Boolean) (SweepResult :type "HitResult Structure (by ref)"))
  (if (== OtherActor (`GameplayStatics.GetPlayerCharacter` 0))
    (`SceneComponent.SetVisibility` (`self.innerInteractIcon`) true false)
    (`SceneComponent.SetVisibility` (`self.outerInteractIcon`) false false)))

(event `self.innerSphereCollision.OnComponentEndOverlap`
  (params (OverlappedComponent :type "PrimitiveComponent Object Reference") (OtherActor :type "Actor Object Reference") (OtherComp :type "PrimitiveComponent Object Reference") (OtherBodyIndex :type Integer))
  (if (== (`GameplayStatics.GetPlayerCharacter` 0) OtherActor)
    (`SceneComponent.SetVisibility` (`self.innerInteractIcon`) false false)
    (`SceneComponent.SetVisibility` (`self.outerInteractIcon`) true false)))

(event `self.outerSphereCollison.OnComponentBeginOverlap`
  (params (OverlappedComponent :type "PrimitiveComponent Object Reference") (OtherActor :type "Actor Object Reference") (OtherComp :type "PrimitiveComponent Object Reference") (OtherBodyIndex :type Integer) (bFromSweep :type Boolean) (SweepResult :type "HitResult Structure (by ref)"))
  (if (== OtherActor (`GameplayStatics.GetPlayerCharacter` 0))
    (`SceneComponent.SetVisibility` (`self.outerInteractIcon`) true false)))

(event `self.outerSphereCollison.OnComponentEndOverlap`
  (params (OverlappedComponent :type "PrimitiveComponent Object Reference") (OtherActor :type "Actor Object Reference") (OtherComp :type "PrimitiveComponent Object Reference") (OtherBodyIndex :type Integer))
  (if (== (`GameplayStatics.GetPlayerCharacter` 0) OtherActor)
    (`SceneComponent.SetVisibility` (`self.outerInteractIcon`) false false)))

(fn `UserConstructionScript`
  (`SphereComponent.SetSphereRadius` (`self.innerSphereCollision`) (`self.innerSphereRadius`) true)
  (`SphereComponent.SetSphereRadius` (`self.outerSphereCollison`) (`self.outerSphereRadius`) true))