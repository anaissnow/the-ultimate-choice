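; BP_Statue is a moving statue hazard that hurts the first-person character on contact.
; On BeginPlay it finds a BP_Path in the level, plays a rock-sliding sound and starts a Timeline that moves and rotates it along the path's spline.
; Actor overlap directly reduces the character's HealthValue, while a separate Box overlap calls ApplyDamage on the character.
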(event `self.ReceiveActorBeginOverlap`
  (params (OtherActor :type "Actor Object Reference"))
  (bind _asbp_first_person_character (cast `/Game/YueErn/YE_Blueprints/BP_FirstPersonCharacter` OtherActor))
  (set `/Game/YueErn/YE_Blueprints/BP_FirstPersonCharacter.HealthValue` (- (`/Game/YueErn/YE_Blueprints/BP_FirstPersonCharacter.HealthValue` _asbp_first_person_character) 0.2) _asbp_first_person_character))

(event `self.ReceiveBeginPlay`
  (bind _returnvalue (`GameplayStatics.GetActorOfClass` "/Game/YueErn/YE_Blueprints/BP_Path.BP_Path_C"))
  (set `self.Path` _returnvalue)
  (`self.Start Moving`)
  (`GameplayStatics.PlaySound2D` "/Game/Sound_Effect/Rock_Sliding_attenuation_.Rock_Sliding_attenuation_" 1.0 1.0 0.0 null null))

(event `Start Moving`
  (bind (_direction _alpha) (`Timeline|Timeline`)
    (:`Update`
      (bind (_returnvalue_location _returnvalue_rotation) (`KismetMathLibrary.BreakTransform` (`SplineComponent.GetTransformAtDistanceAlongSpline` (`/Game/YueErn/YE_Blueprints/BP_Path.Spline` (`self.Path`)) (`KismetMathLibrary.Lerp` 0.0 (`SplineComponent.GetSplineLength` (`/Game/YueErn/YE_Blueprints/BP_Path.Spline` (`self.Path`))) _alpha) "World" false)))
      (`self.K2_SetActorLocationAndRotation` _returnvalue_location _returnvalue_rotation))))

(event `self.Box.OnComponentBeginOverlap`
  (params (OverlappedComponent :type "PrimitiveComponent Object Reference") (OtherActor :type "Actor Object Reference") (OtherComp :type "PrimitiveComponent Object Reference") (OtherBodyIndex :type Integer) (bFromSweep :type Boolean) (SweepResult :type "HitResult Structure (by ref)"))
  (bind _asbp_first_person_character (cast `/Game/YueErn/YE_Blueprints/BP_FirstPersonCharacter` OtherActor))
  (`GameplayStatics.ApplyDamage` _asbp_first_person_character 5.0))

(fn `UserConstructionScript`)